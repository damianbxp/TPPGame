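; Portable toilet prop Blueprint with an automatic swinging door and a color-cycling point light.
; Overlapping the Box plays a timeline that yaws the SMPortapotty03 mesh, and leaving it reverses the swing.
; A second timeline, started on BeginPlay, lerps the light from its current color to a target, then picks a random RGB target and replays endlessly.
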(event `self.ReceiveBeginPlay`
  (bind _returnvalue (`LightComponentBase.GetLightColor` (`self.PointLight`)))
  (set `self.OldColor` _returnvalue)
  (bind (_direction _newtrack_0) (`Timeline|Timeline_0` :!label _label)
    (:`Update`
      (`LightComponent.SetLightColor` (`self.PointLight`) (`KismetMathLibrary.LinearColorLerp` (`self.OldColor`) (`self.NewColor`) _newtrack_0) true))
    (:`Finished`
      (set `self.OldColor` _returnvalue)
      (set `self.NewColor` (`KismetMathLibrary.MakeColor` (`KismetMathLibrary.RandomFloatInRange` 0.0 1.0) (`KismetMathLibrary.RandomFloatInRange` 0.0 1.0) (`KismetMathLibrary.RandomFloatInRange` 0.0 1.0)))
      (goto _label :!via `PlayFromStart`))))

(event `self.Box.OnComponentBeginOverlap`
  (params (OverlappedComponent :type "PrimitiveComponent Object Reference") (OtherActor :type "Actor Object Reference") (OtherComp :type "PrimitiveComponent Object Reference") (OtherBodyIndex :type Integer) (bFromSweep :type Boolean) (SweepResult :type "HitResult Structure (by ref)"))
  (bind (_direction _newtrack_0) (`Timeline|Timeline` :!label _label_2)
    (:`Update`
      (`SceneComponent.K2_SetRelativeRotation` (`self.SM_Portapotty_03`) (`KismetMathLibrary.MakeRotator` 0.0 0.0 _newtrack_0) false false))))

(event `self.Box.OnComponentEndOverlap`
  (params (OverlappedComponent :type "PrimitiveComponent Object Reference") (OtherActor :type "Actor Object Reference") (OtherComp :type "PrimitiveComponent Object Reference") (OtherBodyIndex :type Integer))
  (goto _label_2 :!via `Reverse`))

(fn `UserConstructionScript`)