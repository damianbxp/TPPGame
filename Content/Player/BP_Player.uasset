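; Player Blueprint that routes input to the ACBuildingSystem component for picking up, adjusting and placing building actors.
; E interacts, or rotates a held building opposite to Q; R resets rotation, X restores the old position, wheel zooms and left click ends interaction.
; Held rotation repeats through Gate and Delay loops.
; SpawnActorAndUse, when nothing is held, spawns a given class ahead of the view through a server event and immediately interacts with it.
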(event `self.ReceiveBeginPlay`
  ;[1 0.6517 0.3191] Preparing Variables
  (`/Game/BuildingSystem/Blueprint/ActorComponent/AC_BuildingSystem.PrepareVeriables` (`self.AC_BuildingSystem`) (`self.FollowCamera`)))

(event `Key|E`
  (params (Key :type "Key Structure"))
  (bind _ac_buildingsystem (`self.AC_BuildingSystem`))
  ;[1 0.6517 0.3191] Interact and rotate right
  (:`Pressed`
    (`/Game/BuildingSystem/Blueprint/ActorComponent/AC_BuildingSystem.As BP Master Building` _ac_buildingsystem
      (:`then`
        (`|ExecutionSequence`
          (:`then_0`
            (goto _label :!via `Open`))
          (:`then_1`
            (`/Engine/EditorBlueprintResources/StandardMacros.Gate` true :!label _label
              (:`Exit`
                (`/Game/BuildingSystem/Blueprint/ActorComponent/AC_BuildingSystem.RotationInteract` (`self.AC_BuildingSystem`) 2.5)
                (`KismetSystemLibrary.Delay` 0.02)
                (goto _label))))))
      (:`else`
        (`/Game/BuildingSystem/Blueprint/ActorComponent/AC_BuildingSystem.InteractServer` _ac_buildingsystem null))))
  (:`Released`
    (goto _label :!via `Close`)))

(event `Key|Q`
  (params (Key :type "Key Structure"))
  (bind _ac_buildingsystem (`self.AC_BuildingSystem`))
  ;[1 0.6517 0.3191] Rotate left
  (:`Pressed`
    (`/Game/BuildingSystem/Blueprint/ActorComponent/AC_BuildingSystem.As BP Master Building` _ac_buildingsystem
      (:`then`
        (`|ExecutionSequence`
          (:`then_0`
            (goto _label_2 :!via `Open`))
          (:`then_1`
            (`/Engine/EditorBlueprintResources/StandardMacros.Gate` true :!label _label_2
              (:`Exit`
                (`/Game/BuildingSystem/Blueprint/ActorComponent/AC_BuildingSystem.RotationInteract` _ac_buildingsystem -2.5)
                (`KismetSystemLibrary.Delay` 0.02)
                (goto _label_2))))))
      (:`else`)))
  (:`Released`
    (goto _label_2 :!via `Close`)))

(event `Key|R`
  (params (Key :type "Key Structure"))
  (bind _ac_buildingsystem (`self.AC_BuildingSystem`))
  ;[1 0.6517 0.3191] Reset rotation
  (:`Pressed`
    (`/Game/BuildingSystem/Blueprint/ActorComponent/AC_BuildingSystem.As BP Master Building` _ac_buildingsystem
      (:`then`
        (`/Game/BuildingSystem/Blueprint/ActorComponent/AC_BuildingSystem.ResetRotation` _ac_buildingsystem))
      (:`else`))))

(event `Key|X`
  (params (Key :type "Key Structure"))
  (bind _ac_buildingsystem (`self.AC_BuildingSystem`))
  ;[1 0.6517 0.3191] Old Position
  (:`Pressed`
    (`/Game/BuildingSystem/Blueprint/ActorComponent/AC_BuildingSystem.As BP Master Building` _ac_buildingsystem
      (:`then`
        (`/Game/BuildingSystem/Blueprint/ActorComponent/AC_BuildingSystem.OldPosition` _ac_buildingsystem))
      (:`else`))))

(event `Key|LeftMouseButton`
  (params (Key :type "Key Structure"))
  (bind _ac_buildingsystem (`self.AC_BuildingSystem`))
  ;[1 0.6517 0.3191] End the interaction
  (:`Pressed`
    (`/Game/BuildingSystem/Blueprint/ActorComponent/AC_BuildingSystem.As BP Master Building` _ac_buildingsystem
      (:`then`
        (`/Game/BuildingSystem/Blueprint/ActorComponent/AC_BuildingSystem.EndInteractServer` _ac_buildingsystem))
      (:`else`))))

(event `InputAxisKey|MouseWheelAxis`
  (params (AxisValue :type "Float (single-precision)"))
  ;[1 0.6517 0.3191] Zoom in and out
  (if (!= AxisValue 0.0)
    (`/Game/BuildingSystem/Blueprint/ActorComponent/AC_BuildingSystem.Zoom Out In` (`self.AC_BuildingSystem`) AxisValue)))

(event `SpawnActorAndUse`
  (params (Class :type "Actor Class Reference"))
  ;[1 0.6517 0.3191] Spawn and use it immediately.
  (`/Game/BuildingSystem/Blueprint/ActorComponent/AC_BuildingSystem.As BP Master Building` (`self.AC_BuildingSystem`)
    (:`then`)
    (:`else`
      (`self.SpawnActorAndUseServer` Class))))

(event `Key|F`
  (params (Key :type "Key Structure"))
  ;[1 0.6517 0.3191] Spawn and use it immediately.
  ;;[1 0 0] To use it, trigger this function and give the building actor class you want it to spawn.
)

(event `SpawnActorAndUseServer`
  (params (Class :type "Actor Class Reference"))
  (bind _ac_buildingsystem (`self.AC_BuildingSystem`))
  ;[1 0.6517 0.3191] Spawn and use it immediately.
  (bind _returnvalue (`|SpawnActorFromClass` Class (`KismetMathLibrary.MakeTransform` (+ (`/Game/BuildingSystem/Blueprint/ActorComponent/AC_BuildingSystem.WorldLoc` _ac_buildingsystem) (* (`KismetMathLibrary.GetForwardVector` (`/Game/BuildingSystem/Blueprint/ActorComponent/AC_BuildingSystem.WorldRot` _ac_buildingsystem)) 250.0))) "Undefined" "SelectDefaultAtRuntime" null null))
  (`KismetSystemLibrary.Delay` 0.0)
  (bind _asbp_master_building (cast `/Game/BuildingSystem/Blueprint/Actor/BP_Master_Building` _returnvalue :!pure true))
  (`/Game/BuildingSystem/Blueprint/Actor/BP_Master_Building.CastHiddenShadowMulti` _asbp_master_building)
  (`/Game/BuildingSystem/Blueprint/ActorComponent/AC_BuildingSystem.InteractServer` (`self.AC_BuildingSystem`) _asbp_master_building))

(fn `UserConstructionScript`)